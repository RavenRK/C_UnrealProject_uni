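; BP_ElecProJ is an electric player projectile that supplies blue slash Niagara effects and zap sounds for firing and impact.
; BeginPlay triggers the spawn feedback, playing the muzzle effect and shot sound at the actor's transform.
; A separate OnHitFeedBack event plays the hit effect and sound the same way.
; The graph holds only this cosmetic feedback, with no movement, damage or call to the hit event.
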(event Custom|PlayerFeedbackOnbeginplay
  (bind _returnvalue (Transformation|GetActorLocation))
  ;[0.15 0.15 0.15 0.5] PLayer FeedBack On Spawn
  (Niagara|SpawnSystematLocation "/Game/Player/Projectiles/elec/NS_Muzzle_Slash01_Blue.NS_Muzzle_Slash01_Blue" _returnvalue (Transformation|GetActorRotation))
  (Audio|PlaySoundatLocation "/Game/Sound/elecShot.elecShot" _returnvalue "0, 0, 0" 1.0 1.0 0.0 0 0 0 0))

(event EventBeginPlay
  (CallFunction|PlayerFeedbackOnbeginplay))

(event EventOnHitFeedBack
  (bind _returnvalue (Transformation|GetActorLocation))
  ;[0.15 0.15 0.15 0.5] VFX to play when dead
  (Niagara|SpawnSystematLocation "/Game/Player/Projectiles/elec/NS_Hit_Slash01_Blue.NS_Hit_Slash01_Blue" _returnvalue (Transformation|GetActorRotation))
  (Audio|PlaySoundatLocation "/Game/Sound/zaphit.zaphit" _returnvalue "0, 0, 0" 1.0 1.0 0.0 0 0 0 0))

(fn ConstructionScript)