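; BP_FireProJ is the player's fire projectile Blueprint, providing the fireball's spawn and hit feedback.
; BeginPlay calls a feedback event that spawns an orange muzzle effect and plays a shot sound at the actor's transform.
; OnHitFeedBack spawns the matching hit effect with an impact sound; nothing in this file calls it, and no movement or damage logic appears here.
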(event Custom|PlayerFeedbackOnbeginplay
  (bind _returnvalue (Transformation|GetActorLocation))
  ;[0.15 0.15 0.15 0.5] PLayer FeedBack On Spawn
  (Niagara|SpawnSystematLocation "/Game/Player/Projectiles/VFX/Fire/NS_Muzzle_Fireball04_Orange.NS_Muzzle_Fireball04_Orange" _returnvalue (Transformation|GetActorRotation))
  (Audio|PlaySoundatLocation "/Game/Sound/shotsound_lowbase.shotsound_lowbase" _returnvalue "0, 0, 0" 1.0 1.0 0.0 0 0 0 0))

(event EventBeginPlay
  (CallFunction|PlayerFeedbackOnbeginplay))

(event EventOnHitFeedBack
  (bind _returnvalue (Transformation|GetActorLocation))
  ;[0.15 0.15 0.15 0.5] VFX to play when dead
  (Niagara|SpawnSystematLocation "/Game/Player/Projectiles/VFX/Fire/NS_Hit_Fireball04_Orange.NS_Hit_Fireball04_Orange" _returnvalue (Transformation|GetActorRotation))
  (Audio|PlaySoundatLocation "/Game/Sound/fire-land224089.fire-land224089" _returnvalue "0, 0, 0" 1.0 1.0 0.0 0 0 0 0))

(fn ConstructionScript)