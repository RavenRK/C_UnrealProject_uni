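; BP_IceProJ is the player's ice projectile Blueprint, supplying the visual and audio feedback for the shot.
; On BeginPlay it spawns a blue ice spike muzzle Niagara effect and plays the shot sound at its own location.
; A separate OnHitFeedBack event spawns the impact effect and glass-break sound; nothing in this graph calls it, and no movement or damage logic appears here.
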(event Custom|PlayerFeedbackOnbeginplay
  (bind _returnvalue (Transformation|GetActorLocation))
  ;[0.15 0.15 0.15 0.5] PLayer FeedBack On Spawn
  (Niagara|SpawnSystematLocation "/Game/Player/Projectiles/VFX/Ice/NS_Muzzle_IceSpike01_Blue.NS_Muzzle_IceSpike01_Blue" _returnvalue (Transformation|GetActorRotation))
  (Audio|PlaySoundatLocation "/Game/Sound/iceShot.iceShot" _returnvalue "0, 0, 0" 1.0 1.0 0.0 0 0 0 0))

(event EventBeginPlay
  (CallFunction|PlayerFeedbackOnbeginplay))

(event EventOnHitFeedBack
  (bind _returnvalue (Transformation|GetActorLocation))
  ;[0.15 0.15 0.15 0.5] VFX to play when dead
  (Niagara|SpawnSystematLocation "/Game/Player/Projectiles/VFX/Ice/NS_Hit_IceSpike01_Blue.NS_Hit_IceSpike01_Blue" _returnvalue (Transformation|GetActorRotation))
  (Audio|PlaySoundatLocation "/Game/Sound/GlassBreakIceShot.GlassBreakIceShot" _returnvalue "0, 0, 0" 1.0 1.0 0.0 0 0 0 0))

(fn ConstructionScript)